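; BigPeg_BP is a clickable peg actor that opens a color selector widget when clicked.
; On BeginPlay it creates its own Big_Peg_Color_Selector for the first player, hands it a reference to the peg and adds it to the viewport hidden.
; A click calls BigPegOnClick, which, only if the peg is enabled, shows the selector and disables the peg.
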(event `self.ReceiveBeginPlay`
  ;[1 1 1] Sets up color selector
  (bind _returnvalue (`|CreateWidget` "/Game/Blueprints/Big_Peg_Color_Selector.Big_Peg_Color_Selector_C" (`GameplayStatics.GetPlayerController` 0)))
  (bind _output_get (set `self.ColorSelector` _returnvalue))
  (set `/Game/Blueprints/Big_Peg_Color_Selector.BigPeg` self _output_get)
  (`UserWidget.AddToViewport` _output_get 1)
  (`Widget.SetVisibility` _output_get "Hidden"))

(event `self.ReceiveActorOnClicked`
  (params (ButtonPressed :type "Key Structure"))
  (`self.BigPegOnClick`))

(fn `BigPegOnClick`
  (bind _returnvalue (`self.GetPegEnabled`))
  (if _returnvalue
    (`Widget.SetVisibility` (`self.ColorSelector`) "Visible")
    (`self.SetPegEnabled` false))
  (return))

(fn `UserConstructionScript`)